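; World audio manager Blueprint that plays, pauses and stops 2D music and spawns 2D sound effects.
; StartMusic stores the spawned component, flags music as playing and binds its finished event to clear that state.
; StopMusic stops immediately or runs a timeline lerping volume toward zero, using FadeDurration as play rate and never calling Stop.
; Sound effects are appended to CurrentlyPlayingSFX, with no removal.
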(event Custom|Bind%20MusicStop%20Event
  (params (Audio%20Component%20Of%20Music :type Audio%20Component%20Object%20Reference))
  ;[1 1 1] Naturally Stops
  (EventDispatchers|BindEventtoOnAudioFinished Audio%20Component%20Of%20Music (delegate Custom|On%20Finished)))

(event Custom|On%20Finished
  ;[1 1 1] Naturally Stops
  (Audio|Components|Audio|SetSound (Variables|Default|GetCurrent%20Playing%20Music) 0)
  (Variables|Default|SetIs%20Music%20Playing false))

(event Custom|Stop%20Music
  (params (Fade? :type Boolean) (Fade%20durration :type Float%20%28double-precision%29))
  (bind _current_playing_music (Variables|Default|GetCurrent%20Playing%20Music))
  ;[1 1 1] Forced Stop
  (if Fade?
    (Components|Timeline|SetPlayRate (Variables|Default|GetFade%20Music) Fade%20durration)
    (bind _newtrack_0 (Timeline|Fade%20Music PlayFromStart)
      (:Update
        (Variables|/Script/Engine.AudioComponent|SetVolumeMultiplier _current_playing_music (Math|Float|Lerp (Variables|/Script/Engine.AudioComponent|GetVolumeMultiplier _current_playing_music) 0.0 _newtrack_0)))
      (:Finished
        (Variables|Default|SetIs%20Music%20Playing false)))
    (else
      (Audio|Components|Audio|Stop _current_playing_music)
      (Variables|Default|SetIs%20Music%20Playing false))))

(event EventBeginPlay)

(event Collision|EventActorBeginOverlap
  (params (OtherActor :type Actor%20Object%20Reference)))

(fn ConstructionScript)

(fn StartMusic
  (params (Music%20to%20Play :type Sound%20Wave%20Object%20Reference) (VolumeMultiplier :type Float%20%28single-precision%29) (PitchMultiplier :type Float%20%28single-precision%29) (StartTime :type Float%20%28single-precision%29) (ConcurrencySettings :type Sound%20Concurrency%20Object%20Reference) (bPersistAcrossLevelTransition :type Boolean) (bAutoDestroy :type Boolean))
  (bind _returnvalue (Audio|SpawnSound2D Music%20to%20Play VolumeMultiplier PitchMultiplier StartTime ConcurrencySettings bPersistAcrossLevelTransition bAutoDestroy))
  (Variables|Default|SetIs%20Music%20Playing true)
  (Variables|Default|SetCurrent%20Playing%20Music _returnvalue)
  (CallFunction|BindMusicStopEvent _returnvalue))

(fn PausePlayMusic
  (params (Option :type E_Play_Pause%20Enum :default "NewEnumerator0"))
  (Class|AudioComponent|SetPaused (Variables|Default|GetCurrent%20Playing%20Music) (Utilities|Select :Index Option :NewEnumerator0 false :NewEnumerator1 true :NewEnumerator2 false)))

(fn PlaySoundEffect
  (params (NewParamSFX :type Sound%20Wave%20Object%20Reference) (VolumeMultiplier :type Float%20%28single-precision%29) (PitchMultiplier :type Float%20%28single-precision%29) (StartTime :type Float%20%28single-precision%29) (ConcurrencySettings :type Sound%20Concurrency%20Object%20Reference) (bPersistAcrossLevelTransition :type Boolean) (bAutoDestroy :type Boolean))
  (bind _returnvalue (Audio|SpawnSound2D NewParamSFX VolumeMultiplier PitchMultiplier StartTime ConcurrencySettings bPersistAcrossLevelTransition bAutoDestroy))
  (Utilities|Array|Add (Variables|Default|GetCurrently%20Playing%20SFX) _returnvalue))