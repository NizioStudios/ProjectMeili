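; BP_SecondWall1 is a breakable wall that shatters on its BreakWall event and then notifies the critter character.
; BreakWall enables physics on three geometry collection components and, after a short delay, shoves them with a large impulse along negative Y.
; Several seconds later it calls WallBrokenTransitionBack on BP_CritterCharacter, found by class lookup, then destroys itself.
; Nothing in this graph triggers BreakWall, and BeginPlay is empty.
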(event Custom|Break%20Wall
  (bind _geometrycollection1 (Variables|Default|GetGeometryCollection1))
  (Physics|SetSimulatePhysics _geometrycollection1 true)
  (Utilities|FlowControl|Delay 0.1)
  (Physics|AddImpulse _geometrycollection1 "0.000000,-10000000.000000,0.000000" "None" false)
  (Utilities|FlowControl|Delay 6.0)
  (bind _returnvalue (Actor|GetActorOfClass "/Game/GlobalLogic/Player/BP_CritterCharacter.BP_CritterCharacter_C"))
  (Default|WallBroken,TransitionBack _returnvalue)
  (Utilities|FlowControl|Delay 1.0)
  (Actor|DestroyActor))

(event Collision|EventActorBeginOverlap
  (params (OtherActor :type Actor%20Object%20Reference)))

(event EventTick
  (params (DeltaSeconds :type Float%20%28single-precision%29)))

(event EventBeginPlay)

(fn ConstructionScript)