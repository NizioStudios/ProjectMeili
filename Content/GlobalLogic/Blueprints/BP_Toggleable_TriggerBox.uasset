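; Toggleable trigger box Blueprint whose pawn overlap detection can be switched on or off.
; The construction script shows or hides the box outline in game and sets a text label from a volume description.
; SetCollisionState switches the box's Pawn channel response between Overlap and Ignore.
; The event graph holds no active logic, so this Blueprint defines no overlap reaction itself.
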(event EventBeginPlay)

(event Collision|EventActorBeginOverlap
  (params (OtherActor :type Actor%20Object%20Reference)))

(event EventTick
  (params (DeltaSeconds :type Float%20%28single-precision%29)))

(fn ConstructionScript
  (Development|SetHiddeninGame (Variables|Default|GetTriggerBox) (not (Variables|Default|GetOutline%20Visble?)) false)
  (Rendering|Components|TextRender|SetText (Variables|Default|GetTextRender) (Utilities|Text|ToText(String) (Variables|Default|GetVolume%20Description))))

(fn SetCollisionState
  (params (Enable%20or%20Disable :type E_ActionStatesEnableorDisable%20Enum :default "NewEnumerator0"))
  (Collision|SetCollisionResponsetoChannel (Variables|Default|GetTriggerBox) "ECC_Pawn" (Utilities|Select :Index Enable%20or%20Disable :NewEnumerator0 "ECR_Overlap" :NewEnumerator1 "ECR_Ignore")))