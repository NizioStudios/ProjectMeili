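; BP_SaveInteract is an interactable, apparently a save point, that flickers a point light as visual feedback when the player interacts with it.
; Its OnInteract override runs a counted Delay loop through a FlipFlop to toggle the light's visibility, then hides the light and resets the counter.
; The graph contains only this effect, with no save logic of its own.
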(event EventBeginPlay
  ;[1 1 1] Constructeur
  (|CallParentFunction) ; This node is disabled and will not be called.\nDrag off pins to build functionality.
)

(event EventOnInteract
  (bind _pointlight (Variables|Default|GetPointLight))
  ;[1 1 1] Override OnInteract - Make an effect on save
  (Variables|Default|SetNumSaveEffect 0)
  (Utilities|FlowControl|Delay 0.05 :!label _label)
  (Utilities|FlowControl|FlipFlop
    (:A
      (Rendering|SetVisibility _pointlight true false))
    (:B
      (Rendering|SetVisibility _pointlight false false)))
  (if (<= (Variables|Default|GetNumSaveEffect) 10)
    (Math|Integer|IncrementInt (Variables|Default|GetNumSaveEffect)
      (:%20%20
        (goto _label)))
    (else
      (Rendering|SetVisibility (Variables|Default|GetPointLight) false false)
      (Variables|Default|SetNumSaveEffect 0))))

(fn ConstructionScript
  (|CallParentFunction))