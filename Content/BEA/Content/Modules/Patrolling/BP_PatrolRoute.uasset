(event EventBeginPlay
  ;[0 0 0] Create all patrol points & start debug timer
  (CallFunction|CreatePatrolPoints)
  ;;[1 0.9852 0] Destroy spline after point data is extracted
  (Components|DestroyComponent (Variables|Default|GetPatrol%20Route%20Spline))
  (Default|CallOnSplineRemoved)
  (if (Variables|Patrol|GetDraw%20Route%20Debug)
    (Utilities|Time|SetTimerbyFunctionName 0 "Draw Debug" 1e+02 true false -1e+02)))

(fn ConstructionScript
  ;[0 0 0] Make sure spline is linear at all times
  (CallFunction|MakeLinearSpline))

(fn MakeLinearSpline
  (bind _patrol_route_spline (Variables|Default|GetPatrol%20Route%20Spline))
  ;[0 0 0] Make sure all spline points are aligned as linear and the route is closed
  (bind _index (Utilities|LoopSplinePoints)
    (:Finish
      (Spline|SetClosedLoop _patrol_route_spline true false)
      (Spline|UpdateSpline _patrol_route_spline)
      (return))
    (:Iteration
      (Spline|SetSplinePointType (Variables|Default|GetPatrol%20Route%20Spline) _index "Linear" false))))

(fn GetNextPatrolPoint
  (params (Index :type Integer))
  ;[0 0 0] Check if the current index is the last index
  (if (== Index (Utilities|Array|LastIndex (Variables|Patrol|GetPoints)))
    ;[0 0 0] Jump back to first point
    (return (Utilities|Array|Get(acopy) (Variables|Patrol|GetPoints)))
    (else
      ;[0 0 0] Return the next point
      (bind _result (Math|Integer|IncrementInt Index)
        (:%20%20
          (return (Utilities|Array|Get(acopy) (Variables|Patrol|GetPoints) _result)))))))

(fn CreatePatrolPoints
  ;[0 0 0] Create internal array of patrol point data
  (bind _index (Utilities|LoopSplinePoints)
    (:Finish
      (CallFunction|ReversePoints)
      (Default|CallOnPointsCreated (Variables|Patrol|GetPoints)))
    (:Iteration
      (bind _output_get (LocalVariables|SetIndex _index))
      (LocalVariables|SetLocation (Spline|GetLocationatSplinePoint (Variables|Default|GetPatrol%20Route%20Spline) _output_get "World"))
      (Utilities|Array|Add (Variables|Patrol|GetPoints) (Utilities|Struct|MakeF_PatrolPoint (LocalVariables|GetIndex) (LocalVariables|GetIndex) (LocalVariables|GetLocation))))))

(fn GetPointbyDistance
  (params (Origin :type Vector))
  ;[0 0 0] Get the first patrol point if valid
  (if (Utilities|Array|IsEmpty (Variables|Patrol|GetPoints))
    (return false "")
    (else
      ;;[1 0.7605 0] Get the neares point
      (Utilities|FlowControl|Sequence
        (:then_0
          (for (_array_element _array_index) (Variables|Patrol|GetPoints)
            (if (< (Math|Vector|Distance(Vector) Origin (.WorldLocation (Utilities|Struct|BreakF_PatrolPoint _array_element))) (LocalVariables|GetDistance))
              (LocalVariables|SetSelection _array_index)
              (LocalVariables|SetDistance (Math|Vector|Distance(Vector) Origin (.WorldLocation (Utilities|Struct|BreakF_PatrolPoint _array_element)))))))
        (:then_1
          (return true (Utilities|Array|Get(acopy) (Variables|Patrol|GetPoints) (LocalVariables|GetSelection))))))))

(fn ReversePoints
  ;[0 0 0] Reverse points if route is reversed
  (switch Utilities|FlowControl|Switch|SwitchonE_RouteDirection (Variables|Patrol|GetSpline%20Direction)
    (:NewEnumerator0
      (return))
    (:NewEnumerator1
      (Utilities|Array|Reverse (Variables|Patrol|GetPoints))
      (for (_array_element _array_index) (Variables|Patrol|GetPoints)
        (Utilities|Array|Add (LocalVariables|GetNew%20Points) (Utilities|Struct|MakeF_PatrolPoint _array_index (.SplineIndex (Utilities|Struct|BreakF_PatrolPoint _array_element)) (.WorldLocation (Utilities|Struct|BreakF_PatrolPoint _array_element)))))
      (Variables|Patrol|SetPoints (LocalVariables|GetNew%20Points)))))

(fn DrawDebug
  ;[0 0 0] Draw Debug Shapes
  (CallFunction|DrawDebugRoute (Variables|Patrol|GetPoints) 1e+02))