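; Combat component that runs its owner's attacks, loading them from a config asset obtained through BPI_AgentProvider.
; PerformAttack picks an off-cooldown attack by weighted random, plays its montage and records its cooldown, or notifies the game controller if none is available.
; ToggleCombatSystem switches child-actor hitboxes, initializing them with the active attack's damage data.
; Montage end fires the finished dispatcher, deactivates the system and clears the active attack.
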(event Custom|On%20Config%20Set
  ;[0 0 0] Prepare attacks after config loaded
  (Internal|PrepareAttacks))

(event Custom|Montage%20Start
  (params (Duration :type Float%20%28double-precision%29) (Anim%20Instance :type Anim%20Instance%20Object%20Reference))
  ;[0 0 0] Called when the attack montage started. Binds to end of montage & calls dispatcher
  (Utilities|IsValid Anim%20Instance
    (:Is%20Valid
      (if (> Duration 0.0)
        (Variables|Attacks|SetCurrent%20Anim%20Instance Anim%20Instance)
        (EventDispatchers|BindEventtoOnMontageEnded Anim%20Instance (delegate Custom|Attack%20Montage%20Ended))
        (Default|CallOnAttackStarted)))))

(event Custom|Attack%20Montage%20Ended
  (params (Montage :type Anim%20Montage%20Object%20Reference) (bInterrupted :type Boolean))
  ;[0 0 0] Called when the attack montage stopped. Calls dispatcher and makes sure the combat system is inactive
  (if (== Montage (.AttackMontage (Utilities|Struct|BreakF_AttackData (Default|GetAttackData (Variables|Attacks|GetActive%20Attack)))))
    (Utilities|IsValid (Variables|Attacks|GetCurrent%20Anim%20Instance)
      (:Is%20Valid
        (EventDispatchers|UnbindEventfromOnMontageEnded (Variables|Attacks|GetCurrent%20Anim%20Instance) (delegate Custom|Attack%20Montage%20Ended))
        (Default|CallOnAttackFinsihed)
        (CallFunction|ToggleCombatSystem false)
        ;;[0 0 0] Nullify active attack after deactivation
        (Variables|Attacks|SetActive%20Attack 0)))))

(event EventBeginPlay
  ;[0 0 0] Initialize the combat system, get config, deactivate hitboxes
  (Internal|GetConfig)
  (bind _aschild_actor_component (|IterateColliders)
    (:Loop%20Body
      (Components|Activation|SetActive _aschild_actor_component false false))))

(fn GetConfig
  (bind _returnvalue (Components|GetOwner))
  ;[0 0 0] Request config asset from owner using interface
  (if (Utilities|DoesObjectImplementInterface _returnvalue "/Game/BEA/Content/Misc/BPI_AgentProvider.BPI_AgentProvider_C")
    (bind (_success _config) (Class|BPIAgentProvider|RequestConfigAsset(Message) _returnvalue))
    (if _success
      (Variables|Default|SetConfig _config)
      (CallFunction|OnConfigSet)
      (return))))

(fn PrepareAttacks
  ;[0 0 0] Get attacks from config. Already sorted
  (bind _output_get (Variables|Attacks|SetAttacks (Utilities|Struct|BreakF_CombatSettings (Default|GetCombatSettings (Variables|Default|GetConfig)))))
  ;[0 0 0] Sort attacks into map
  (for _array_element _output_get
    (Utilities|Map|Add (Variables|Attacks|GetCooldown%20Register) _array_element -999.0)))

(fn MarkAttackUsed
  (params (Attack :type BP%20Attack%20Config%20Object%20Reference))
  (Utilities|IsValid Attack
    (:Is%20Valid
      ;[0 0 0] Update attack cooldown in map
      (Utilities|Map|Add (Variables|Attacks|GetCooldown%20Register) Attack (+ (.Cooldown (Utilities|Struct|BreakF_AttackData (Default|GetAttackData Attack))) (+ (Utilities|Time|GetGameTimeinSeconds) 0.2))))
    (:Is%20Not%20Valid
      (return))))

(fn PlayAttack
  (params (Attack :type BP%20Attack%20Config%20Object%20Reference))
  (Utilities|FlowControl|Sequence
    (:then_0
      (Utilities|IsValid Attack
        (:Is%20Valid
          ;[0 0 0] Get mesh from owner and start playing attack montage
          (bind _ascharacter (Utilities|Casting|CastToCharacter (Components|GetOwner)))
          (Utilities|IsValid (Variables|/Script/Engine.Character|GetMesh _ascharacter)
            (:Is%20Valid
              (bind _output_get (LocalVariables|SetAnim%20Instance (Components|SkeletalMesh|GetAnimInstance (Variables|/Script/Engine.Character|GetMesh _ascharacter))))
              (bind _returnvalue (Animation|Montage|MontagePlay _output_get (.AttackMontage (Utilities|Struct|BreakF_AttackData (Default|GetAttackData Attack))) 1.0 "Duration" 0.0 true))
              (if (> _returnvalue 0.0)
                (CallFunction|MontageStart _returnvalue (LocalVariables|GetAnim%20Instance))
                (return true)))))))
    (:then_1
      (return false))))

(fn ToggleColliders
  (params (Toggle :type Boolean) (Components :type Array%20of%20Child%20Actor%20Component%20Object%20References) (Colliders :type Array%20of%20BP%20Hitbox%20Object%20References))
  (bind _active_attack (Variables|Attacks|GetActive%20Attack))
  (bind _attack_data (Default|GetAttackData _active_attack))
  (bind (_attackmontage _damagerange _damagetype) (Utilities|Struct|BreakF_AttackData _attack_data))
  (Utilities|FlowControl|Sequence
    (:then_0
      ;[0 0 0] Deactivate / Activate components, based on toggle
      (for _array_element Components
        (Components|Activation|SetActive _array_element Toggle false)))
    (:then_1
      ;[0 0 0] Initialize colliders
      (if Toggle
        (for _array_element_2 Colliders
          (Default|InitializeHitbox _array_element_2 _damagerange _damagetype (Components|GetOwner)))))))

(fn SelectAttack
  (Utilities|FlowControl|Sequence
    (:then_0
      ;[0 0 0] 1.1: Sort out all attacks that do not have an active cooldown
      (Utilities|FlowControl|Sequence
        (:then_0
          (for _array_element (Variables|Attacks|GetAttacks)
            (if (.ReturnValue (Utilities|Map|Find (Variables|Attacks|GetCooldown%20Register) _array_element))
              (if (>= (Utilities|Time|GetGameTimeinSeconds) (.Value (Utilities|Map|Find (Variables|Attacks|GetCooldown%20Register) _array_element)))
                (Utilities|Array|Add (LocalVariables|GetCandidates) _array_element)))))
        (:then_1
          ;[0 0 0] 1.2: Abort if there are no available attacks
          (if (Utilities|Array|IsEmpty (LocalVariables|GetCandidates))
            (return false 0)))))
    (:then_1
      ;[0 0 0] 2.1: Get the combined weight of all available attacks
      (Utilities|FlowControl|Sequence
        (:then_0
          (for _array_element_2 (LocalVariables|GetCandidates)
            (LocalVariables|SetTotal%20Weight (+ (LocalVariables|GetTotal%20Weight) (Math|Float|Clamp(Float) (.Weight (Utilities|Struct|BreakF_AttackData (Default|GetAttackData _array_element_2))))))))
        (:then_1
          ;[0 0 0] 2.2: If all have no weight, return random attack
          (if (<= (LocalVariables|GetTotal%20Weight) (Math|Float|MakeLiteralFloat 0.0))
            (return true (.OutItem (Utilities|Array|Random (LocalVariables|GetCandidates))))))))
    (:then_2
      ;[0 0 0] 3.1: Get a random target weight and then iterate the attacks, accumulating the attack weights. Select the first attack that breaks even.
      (LocalVariables|SetTarget%20Weight (Math|Random|RandomFloatinRange (Math|Float|MakeLiteralFloat 0.0) (LocalVariables|GetTotal%20Weight)))
      (LocalVariables|SetAccquired%20Weight 0.0)
      (for _array_element_3 (LocalVariables|GetCandidates)
        (bind _output_get (LocalVariables|SetAccquired%20Weight (+ (LocalVariables|GetAccquired%20Weight) (Math|Float|Clamp(Float) (.Weight (Utilities|Struct|BreakF_AttackData (Default|GetAttackData _array_element_3)))))))
        (if (>= _output_get (LocalVariables|GetTarget%20Weight))
          (return true _array_element_3))))
    (:then_3
      (return false 0))))

(fn GetCombatComponent
  ;[0 0 0] Return self
  (return self))

(fn PerformAttack
  (Utilities|FlowControl|Sequence
    (:then_0
      ;[1 0 0] Do not perform attack if other is active
      (if (not (Utilities|IsValid (Variables|Attacks|GetActive%20Attack)))
        ;[0 0 0] Select available attack, play & mark as used
        (bind (_success _attack) (Internal|SelectAttack))
        (if _success
          (Internal|PlayAttack _attack)
          (Variables|Attacks|SetActive%20Attack _attack)
          (Internal|MarkAttackUsed _attack)
          (return true)
          (else
            (bind _returnvalue (Actor|GetActorOfClass "/Game/LevelAssets/Epic/StoryAdvTemplate/Blueprints/BP_GameController_New.BP_GameController_New_C"))
            (Default|AttackTriggered _returnvalue)
            (return false)))))
    (:then_1
      (return false))))

(fn ToggleCombatSystem
  (params (Toggle :type Boolean))
  (Utilities|FlowControl|Sequence
    (:then_0
      ;[1 0 0] Make sure that the wanted state is not the same as the current state
      (if (!= Toggle (Variables|Default|GetState))
        ;[0 0 0] Set new state , get colliders, get components, toggle colliders
        (bind _output_get (Variables|Default|SetState Toggle))
        (|GetComponents&Collider)
        (Internal|ToggleColliders _output_get (LocalVariables|GetComponents) (LocalVariables|GetCollider))))
    (:then_1
      (return (Variables|Default|GetState)))))