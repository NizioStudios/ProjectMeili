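; Anim notify state that switches the owning actor's combat system on for the duration of an animation window.
; Begin calls ToggleCombatSystem(true) and end calls it with false, both through the BPI_CombatSystem interface.
; A helper finds the BP_CombatSystemT component on the mesh owner and casts it to that interface, reporting failure when none is found.
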(fn ReceivedNotifyBegin
  (params (MeshComp :type Skeletal%20Mesh%20Component%20Object%20Reference) (Animation :type Anim%20Sequence%20Base%20Object%20Reference) (TotalDuration :type Float%20%28single-precision%29) (EventReference :type Anim%20Notify%20Event%20Reference%20Structure%20%28by%20ref%29))
  (bind (_success _combat_interface) (CallFunction|GetCombatInterface MeshComp))
  ;[0 0 0] Activate the combat system when the notify is triggered
  (if _success
    (bind _new_state (Default|ToggleCombatSystem _combat_interface true))
    (return _new_state)
    (else
      (return false))))

(fn ReceivedNotifyEnd
  (params (MeshComp :type Skeletal%20Mesh%20Component%20Object%20Reference) (Animation :type Anim%20Sequence%20Base%20Object%20Reference) (EventReference :type Anim%20Notify%20Event%20Reference%20Structure%20%28by%20ref%29))
  (bind (_success _combat_interface) (CallFunction|GetCombatInterface MeshComp))
  ;[0 0 0] deactivate the combat system when the notify is finished
  (if _success
    (bind _new_state (Default|ToggleCombatSystem _combat_interface false))
    (return _new_state)
    (else
      (return false))))

(fn GetCombatInterface
  (params (Mesh :type Skeletal%20Mesh%20Component%20Object%20Reference))
  (Utilities|FlowControl|Sequence
    (:then_0
      ;[0 0 0] Make sure the owner contains a combat system that uses the proper interface
      (bind _output_get (LocalVariables|SetOwner (Components|GetOwner Mesh)))
      (Utilities|IsValid _output_get
        (:Is%20Valid
          (bind _output_get_2 (LocalVariables|SetCombat%20System%20Component (Actor|GetComponentbyClass _output_get "/Game/BEA/Content/Modules/Combat/BP_CombatSystemT.BP_CombatSystemT_C")))
          (Utilities|IsValid _output_get_2
            (:Is%20Valid
              (bind _asbpi_combat_system (Utilities|Casting|CastToBPI_CombatSystem (LocalVariables|GetCombat%20System%20Component)))
              (return true _asbpi_combat_system))))))
    (:then_1
      (return false 0))))