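; Base Blueprint for enemy characters that manages an overhead healthbar and exposes AI data.
; When its config enables the healthbar, BeginPlay binds the widget to the health system and Tick turns it toward the player camera.
; Reinitalize repeats that setup and reinitializes the combat system.
; Helper functions toggle widget visibility and return the config asset and patrol route with validity flags.
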(event Custom|Reinitalize
  (bind _config (Variables|EnemyConfifuration|GetConfig))
  (bind _config_2 (Variables|EnemyConfifuration|GetConfig))
  (Utilities|FlowControl|Sequence
    (:then_0
      ;[0 0 0] Unreal Events: Initialize Health System
      (CallFunction|InitializeHealthbarWidget))
    (:then_1
      ;[1 0.963 0] Interface Implementations
      ;;[0 1 0.3661] Get the healthbar widget from widget component and perform init logic
      (Utilities|IsValid _config_2
        (:Is%20Valid
          (if (Variables|/Game/BEA/Content/Modules/Config/Agents/Core/BP_EnemyConfig.BP_EnemyConfig_C|GetShow%20Healthbar _config_2)
            (Rendering|SetVisibility (Variables|Default|GetWidget) true false)
            (bind _aswbp_healthbar (Utilities|Casting|CastToWBP_Healthbar (UserInterface|GetWidget (Variables|Default|GetWidget))))
            (Default|SetupHealthbarWidget _aswbp_healthbar (Variables|Default|GetHealth%20System))))))
    (:then_2
      ;;[0 1 0.3682] Constantly rotate the widget to the player camera
      (Utilities|IsValid _config
        (:Is%20Valid
          (if (Variables|/Game/BEA/Content/Modules/Config/Agents/Core/BP_EnemyConfig.BP_EnemyConfig_C|GetShow%20Healthbar _config)
            (Transformation|SetWorldRotation (Variables|Default|GetWidget) (Math|Rotator|FindLookatRotation (Transformation|GetWorldLocation (Variables|Default|GetWidget)) (Transformation|GetWorldLocation (Variables|/Script/Engine.PlayerCameraManager|GetTransformComponent (Game|GetPlayerCameraManager 0)))) false false)))))
    (:then_3
      (Default|Reinit (Variables|Default|GetCombat%20System)))))

(event EventTick
  (params (DeltaSeconds :type Float%20%28single-precision%29))
  ;[0 0 0] Unreal Events: Initialize Health System
  (CallFunction|RotateWidgettoView))

(event EventBeginPlay
  ;[0 0 0] Unreal Events: Initialize Health System
  (CallFunction|InitializeHealthbarWidget))

(event EventInitializeHealthbarWidget
  (bind _config (Variables|EnemyConfifuration|GetConfig))
  ;[1 0.963 0] Interface Implementations
  ;;[0 1 0.3661] Get the healthbar widget from widget component and perform init logic
  (Utilities|IsValid _config
    (:Is%20Valid
      (if (Variables|/Game/BEA/Content/Modules/Config/Agents/Core/BP_EnemyConfig.BP_EnemyConfig_C|GetShow%20Healthbar _config)
        (Rendering|SetVisibility (Variables|Default|GetWidget) true false)
        (bind _aswbp_healthbar (Utilities|Casting|CastToWBP_Healthbar (UserInterface|GetWidget (Variables|Default|GetWidget))))
        (Default|SetupHealthbarWidget _aswbp_healthbar (Variables|Default|GetHealth%20System))))))

(event EventRotateWidgettoView
  (bind _config (Variables|EnemyConfifuration|GetConfig))
  ;[1 0.963 0] Interface Implementations
  ;;[0 1 0.3682] Constantly rotate the widget to the player camera
  (Utilities|IsValid _config
    (:Is%20Valid
      (if (Variables|/Game/BEA/Content/Modules/Config/Agents/Core/BP_EnemyConfig.BP_EnemyConfig_C|GetShow%20Healthbar _config)
        (Transformation|SetWorldRotation (Variables|Default|GetWidget) (Math|Rotator|FindLookatRotation (Transformation|GetWorldLocation (Variables|Default|GetWidget)) (Transformation|GetWorldLocation (Variables|/Script/Engine.PlayerCameraManager|GetTransformComponent (Game|GetPlayerCameraManager 0)))) false false)))))

(fn ConstructionScript)

(fn ToggleHealthWidget
  (params (Wanted%20State :type Boolean))
  ;[0 0 0] Toggle Widget Visibility based on wanted state
  (if (!= Wanted%20State (Class|WidgetComponent|IsWidgetVisible (Variables|Default|GetWidget)))
    (Rendering|SetVisibility (Variables|Default|GetWidget) Wanted%20State false))
  (return (Class|WidgetComponent|IsWidgetVisible (Variables|Default|GetWidget))))

(fn RequestConfigAsset
  (bind _config (Variables|EnemyConfifuration|GetConfig))
  ;[0 0 0] Return the config asset and see if its valid
  (return (Utilities|IsValid _config) _config))

(fn RequestPatrolRoute
  (bind _patrol_route (Variables|EnemyConfifuration|GetPatrol%20Route))
  ;[0 0 0] Return the patrol route and see if its valid
  (return (Utilities|IsValid _patrol_route) _patrol_route))