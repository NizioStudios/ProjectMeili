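; Master interactable computer monitor that builds its widget desktop, lore items and apps from a construct data asset on BeginPlay.
; Interaction, gated by that asset, blends the view to the monitor and swaps player actions, crosshair and HUD for cursor-driven UI input.
; Interacting again, the stop-inspecting input or ReleasePlayerFromComputerCamera blends back to the player, restoring control once the camera blend time elapses.
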(event Custom|Release%20Player%20From%20Computer%20Camera
  (bind _as_bp_pc_mwiplayer_controller (Variables|References|GetAs%20BP%20PC%20MWIPlayer%20Controller))
  (bind _as_bp_pc_mwiplayer_controller_2 (Variables|References|GetAs%20BP%20PC%20MWIPlayer%20Controller))
  ;[0.2188 0 1] Event Interaction
  (Game|Player|SetViewTargetwithBlend (Game|GetPlayerController 0) (Game|GetPlayerCharacter 0) (Variables|/Game/Interactable_Items/0Master_Blueprints/DataAssets/DA_Master_Computer.DA_Master_Computer_C|GetCamera%20Blend%20Time (Variables|ConstructComputer|GetConstruct%20Computer%20Data%20Asset)) "VTBlend_Linear" 0.0 false :!pinned true) ; Transition back to player
  (CallFunction|SetOutlineVisbility "NewEnumerator0")
  (Variables|Bools|SetPlayer%20Focused false) ; Set Player not looking at keypad
  (Variables|/Script/Engine.PlayerController|SetbShowMouseCursor _as_bp_pc_mwiplayer_controller false) ; Hide mouse
  (Default|FadeCrosshairAnim _as_bp_pc_mwiplayer_controller "Reverse" 2.0) ; Fade in crosshair
  (Variables|/Game/PlayerLogic/Blueprints/BP_I_MWInstance.BP_I_MWInstance_C|SetCurrentUIMode (Variables|References|GetAs%20BP%20I%20MWInstance) "NewEnumerator0") ; Set ui mode no menu
  (Input|DisableInput (Game|GetPlayerController 0)) ; Disable player input on keypad
  (Default|SetInteractablesInputContext _as_bp_pc_mwiplayer_controller_2 "NewEnumerator0" "NewEnumerator1") ; Remove interractables input context
  (Utilities|FlowControl|Delay (Variables|/Game/Interactable_Items/0Master_Blueprints/DataAssets/DA_Master_Computer.DA_Master_Computer_C|GetCamera%20Blend%20Time (Variables|ConstructComputer|GetConstruct%20Computer%20Data%20Asset)))
  (Default|EnableEverything (Variables|References|GetAs%20BP%20First%20Person%20Character)) ; Enable player actions
  (Input|SetInputModeGameOnly _as_bp_pc_mwiplayer_controller_2 false)
  (Default|SetGIVisibility (Variables|/Game/LevelAssets/Epic/StoryAdvTemplate/Blueprints/BP_GameController_New.BP_GameController_New_C|GetGalactic%20Interface%20Ref (Variables|References|GetGame%20Controller%20Reference)) "NewEnumerator0")
  (Widget|SetVisibility (UserInterface|GetWidget (Variables|Default|GetKeypress%20Prompt%20Indicator%20Widget)) "Visible"))

(event Input|EnhancedActionEvents|EnhancedInputActionIA_Stop_Inspecting
  (params (ActionValue :type Boolean) (ElapsedSeconds :type Float%20%28double-precision%29) (TriggeredSeconds :type Float%20%28double-precision%29) (InputAction :type Input%20Action%20Object%20Reference :default "/Game/Input/Input_Actions/Interactables/IA_Stop_Inspecting.IA_Stop_Inspecting"))
  (bind _construct_computer_data_asset (Variables|ConstructComputer|GetConstruct%20Computer%20Data%20Asset))
  (bind _as_bp_pc_mwiplayer_controller (Variables|References|GetAs%20BP%20PC%20MWIPlayer%20Controller))
  (bind _keypress_prompt_indicator_widget (Variables|Default|GetKeypress%20Prompt%20Indicator%20Widget))
  (bind _game_controller_reference (Variables|References|GetGame%20Controller%20Reference))
  (bind _construct_computer_data_asset_2 (Variables|ConstructComputer|GetConstruct%20Computer%20Data%20Asset))
  (bind _as_bp_pc_mwiplayer_controller_2 (Variables|References|GetAs%20BP%20PC%20MWIPlayer%20Controller))
  (bind _returnvalue (UserInterface|GetWidget _keypress_prompt_indicator_widget))
  (bind _galactic_interface_ref (Variables|/Game/LevelAssets/Epic/StoryAdvTemplate/Blueprints/BP_GameController_New.BP_GameController_New_C|GetGalactic%20Interface%20Ref _game_controller_reference))
  (bind _camera_blend_time (Variables|/Game/Interactable_Items/0Master_Blueprints/DataAssets/DA_Master_Computer.DA_Master_Computer_C|GetCamera%20Blend%20Time _construct_computer_data_asset))
  (bind _camera_blend_time_2 (Variables|/Game/Interactable_Items/0Master_Blueprints/DataAssets/DA_Master_Computer.DA_Master_Computer_C|GetCamera%20Blend%20Time _construct_computer_data_asset_2))
  ;[0.2188 0 1] Event Interaction
  (:Started
    (if (Variables|Bools|GetPlayer%20Focused) ; Is player looking at keypad
      (Game|Player|SetViewTargetwithBlend (Game|GetPlayerController 0) (Game|GetPlayerCharacter 0) _camera_blend_time_2 "VTBlend_Linear" 0.0 false :!pinned true) ; Transition back to player
      (CallFunction|SetOutlineVisbility "NewEnumerator0")
      (Variables|Bools|SetPlayer%20Focused false) ; Set Player not looking at keypad
      (Variables|/Script/Engine.PlayerController|SetbShowMouseCursor _as_bp_pc_mwiplayer_controller false) ; Hide mouse
      (Default|FadeCrosshairAnim _as_bp_pc_mwiplayer_controller "Reverse" 2.0) ; Fade in crosshair
      (Variables|/Game/PlayerLogic/Blueprints/BP_I_MWInstance.BP_I_MWInstance_C|SetCurrentUIMode (Variables|References|GetAs%20BP%20I%20MWInstance) "NewEnumerator0") ; Set ui mode no menu
      (Input|DisableInput (Game|GetPlayerController 0)) ; Disable player input on keypad
      (Default|SetInteractablesInputContext _as_bp_pc_mwiplayer_controller_2 "NewEnumerator0" "NewEnumerator1") ; Remove interractables input context
      (Utilities|FlowControl|Delay _camera_blend_time)
      (Default|EnableEverything (Variables|References|GetAs%20BP%20First%20Person%20Character)) ; Enable player actions
      (Input|SetInputModeGameOnly _as_bp_pc_mwiplayer_controller_2 false)
      (Default|SetGIVisibility _galactic_interface_ref "NewEnumerator0")
      (Widget|SetVisibility _returnvalue "Visible")
      (else
        (Game|Player|SetViewTargetwithBlend (Game|GetPlayerController 0) self _camera_blend_time_2 "VTBlend_Linear" 0.0 false) ; Transition to computer camera
        (CallFunction|SetOutlineVisbility "NewEnumerator1")
        (Variables|Bools|SetPlayer%20Focused true) ; Set player is looking at keypad
        (Default|FadeCrosshairAnim _as_bp_pc_mwiplayer_controller "Forward" 2.0) ; Fade out crosshair
        (Default|DisableEverything (Variables|References|GetAs%20BP%20First%20Person%20Character)) ; Disable player actions
        (Variables|/Game/PlayerLogic/Blueprints/BP_I_MWInstance.BP_I_MWInstance_C|SetCurrentUIMode (Variables|References|GetAs%20BP%20I%20MWInstance) "NewEnumerator6") ; Set ui mode focusable game object
        (Input|EnableInput (Game|GetPlayerController 0)) ; Enable character input for keypad
        (Default|SetInteractablesInputContext (Variables|References|GetAs%20BP%20PC%20MWIPlayer%20Controller) "NewEnumerator0") ; Add interactables input context
        (Variables|/Script/Engine.PlayerController|SetbShowMouseCursor (Variables|References|GetAs%20BP%20PC%20MWIPlayer%20Controller) true) ; Show mouse cursor
        (Utilities|FlowControl|Delay _camera_blend_time)
        (Input|SetInputModeGameandUI _as_bp_pc_mwiplayer_controller_2 (UserInterface|GetWidget (Variables|Default|GetComputerWidget)) "LockOnCapture" true false)
        (Default|SetGIVisibility _galactic_interface_ref "NewEnumerator0" "NewEnumerator1")
        (Widget|SetVisibility _returnvalue "Hidden")))))

(event Collision|EventActorBeginOverlap
  (params (OtherActor :type Actor%20Object%20Reference))
  (|CallParentFunction OtherActor) ; This node is disabled and will not be called.\nDrag off pins to build functionality.
)

(event EventInteraction
  (params (Is%20Being%20Held :type Boolean) (Key :type Key%20Structure))
  (bind _construct_computer_data_asset (Variables|ConstructComputer|GetConstruct%20Computer%20Data%20Asset))
  (bind _as_bp_pc_mwiplayer_controller (Variables|References|GetAs%20BP%20PC%20MWIPlayer%20Controller))
  (bind _keypress_prompt_indicator_widget (Variables|Default|GetKeypress%20Prompt%20Indicator%20Widget))
  (bind _game_controller_reference (Variables|References|GetGame%20Controller%20Reference))
  (bind _construct_computer_data_asset_2 (Variables|ConstructComputer|GetConstruct%20Computer%20Data%20Asset))
  (bind _as_bp_pc_mwiplayer_controller_2 (Variables|References|GetAs%20BP%20PC%20MWIPlayer%20Controller))
  (bind _returnvalue (UserInterface|GetWidget _keypress_prompt_indicator_widget))
  (bind _galactic_interface_ref (Variables|/Game/LevelAssets/Epic/StoryAdvTemplate/Blueprints/BP_GameController_New.BP_GameController_New_C|GetGalactic%20Interface%20Ref _game_controller_reference))
  (bind _camera_blend_time (Variables|/Game/Interactable_Items/0Master_Blueprints/DataAssets/DA_Master_Computer.DA_Master_Computer_C|GetCamera%20Blend%20Time _construct_computer_data_asset))
  (bind _camera_blend_time_2 (Variables|/Game/Interactable_Items/0Master_Blueprints/DataAssets/DA_Master_Computer.DA_Master_Computer_C|GetCamera%20Blend%20Time _construct_computer_data_asset_2))
  ;[0.2188 0 1] Event Interaction
  (|CallParentFunction Is%20Being%20Held Key)
  (if (Variables|/Game/Interactable_Items/0Master_Blueprints/DataAssets/DA_Master_Computer.DA_Master_Computer_C|GetCan%20Interact%20With%20Computer _construct_computer_data_asset_2) ; Can player interact with keypad
    (if (Variables|Bools|GetPlayer%20Focused) ; Is player looking at keypad
      (Game|Player|SetViewTargetwithBlend (Game|GetPlayerController 0) (Game|GetPlayerCharacter 0) _camera_blend_time_2 "VTBlend_Linear" 0.0 false :!pinned true) ; Transition back to player
      (CallFunction|SetOutlineVisbility "NewEnumerator0")
      (Variables|Bools|SetPlayer%20Focused false) ; Set Player not looking at keypad
      (Variables|/Script/Engine.PlayerController|SetbShowMouseCursor _as_bp_pc_mwiplayer_controller false) ; Hide mouse
      (Default|FadeCrosshairAnim _as_bp_pc_mwiplayer_controller "Reverse" 2.0) ; Fade in crosshair
      (Variables|/Game/PlayerLogic/Blueprints/BP_I_MWInstance.BP_I_MWInstance_C|SetCurrentUIMode (Variables|References|GetAs%20BP%20I%20MWInstance) "NewEnumerator0") ; Set ui mode no menu
      (Input|DisableInput (Game|GetPlayerController 0)) ; Disable player input on keypad
      (Default|SetInteractablesInputContext _as_bp_pc_mwiplayer_controller_2 "NewEnumerator0" "NewEnumerator1") ; Remove interractables input context
      (Utilities|FlowControl|Delay _camera_blend_time)
      (Default|EnableEverything (Variables|References|GetAs%20BP%20First%20Person%20Character)) ; Enable player actions
      (Input|SetInputModeGameOnly _as_bp_pc_mwiplayer_controller_2 false)
      (Default|SetGIVisibility _galactic_interface_ref "NewEnumerator0")
      (Widget|SetVisibility _returnvalue "Visible")
      (else
        (Game|Player|SetViewTargetwithBlend (Game|GetPlayerController 0) self _camera_blend_time_2 "VTBlend_Linear" 0.0 false) ; Transition to computer camera
        (CallFunction|SetOutlineVisbility "NewEnumerator1")
        (Variables|Bools|SetPlayer%20Focused true) ; Set player is looking at keypad
        (Default|FadeCrosshairAnim _as_bp_pc_mwiplayer_controller "Forward" 2.0) ; Fade out crosshair
        (Default|DisableEverything (Variables|References|GetAs%20BP%20First%20Person%20Character)) ; Disable player actions
        (Variables|/Game/PlayerLogic/Blueprints/BP_I_MWInstance.BP_I_MWInstance_C|SetCurrentUIMode (Variables|References|GetAs%20BP%20I%20MWInstance) "NewEnumerator6") ; Set ui mode focusable game object
        (Input|EnableInput (Game|GetPlayerController 0)) ; Enable character input for keypad
        (Default|SetInteractablesInputContext (Variables|References|GetAs%20BP%20PC%20MWIPlayer%20Controller) "NewEnumerator0") ; Add interactables input context
        (Variables|/Script/Engine.PlayerController|SetbShowMouseCursor (Variables|References|GetAs%20BP%20PC%20MWIPlayer%20Controller) true) ; Show mouse cursor
        (Utilities|FlowControl|Delay _camera_blend_time)
        (Input|SetInputModeGameandUI _as_bp_pc_mwiplayer_controller_2 (UserInterface|GetWidget (Variables|Default|GetComputerWidget)) "LockOnCapture" true false)
        (Default|SetGIVisibility _galactic_interface_ref "NewEnumerator0" "NewEnumerator1")
        (Widget|SetVisibility _returnvalue "Hidden")))))

(event EventBeginPlay
  (bind _construct_computer_data_asset (Variables|ConstructComputer|GetConstruct%20Computer%20Data%20Asset))
  ;[1 0.7266 0] Event Begin Play
  (|CallParentFunction)
  (bind _returnvalue (Actor|GetActorOfClass "/Game/LevelAssets/Epic/StoryAdvTemplate/Blueprints/BP_GameController_New.BP_GameController_New_C"))
  (Variables|References|SetGame%20Controller%20Reference _returnvalue)
  (bind _asbp_pc_mwiplayer_controller (Utilities|Casting|CastToBP_PC_MWIPlayerController (Game|GetPlayerController 0)))
  (Variables|References|SetAs%20BP%20PC%20MWIPlayer%20Controller _asbp_pc_mwiplayer_controller) ; Set player controller reference
  (bind _asbp_first_person_character (Utilities|Casting|CastToBP_FirstPersonCharacter (Game|GetPlayerCharacter 0)))
  (Variables|References|SetAs%20BP%20First%20Person%20Character _asbp_first_person_character) ; Set fpc reference
  (bind _asbp_i_mwinstance (Utilities|Casting|CastToBP_I_MWInstance (Game|GetGameInstance)))
  (Variables|References|SetAs%20BP%20I%20MWInstance _asbp_i_mwinstance) ; Set game instance reference
  (bind _aswbp_master_computer_monitor (Utilities|Casting|CastToWBP_Master_Computer_Monitor (UserInterface|GetWidget (Variables|Default|GetComputerWidget))))
  (Variables|References|SetAs%20WBP%20Master%20Computer%20Monitor _aswbp_master_computer_monitor)
  (if (Utilities|IsValid _construct_computer_data_asset)
    (Default|ConstructComputerSystem _aswbp_master_computer_monitor (Variables|/Game/Interactable_Items/0Master_Blueprints/DataAssets/DA_Master_Computer.DA_Master_Computer_C|GetDesktop%20Setup _construct_computer_data_asset) (Variables|/Game/Interactable_Items/0Master_Blueprints/DataAssets/DA_Master_Computer.DA_Master_Computer_C|GetLore%20Items _construct_computer_data_asset) (Variables|/Game/Interactable_Items/0Master_Blueprints/DataAssets/DA_Master_Computer.DA_Master_Computer_C|GetGlobal%20App%20Setup _construct_computer_data_asset) (Variables|References|GetGame%20Controller%20Reference)) ; Construct computer system
    (else
      (CallFunction|PrintDebugData false (Utilities|String|Append (Utilities|String|ToString(Name) (Variables|/Game/Interactable_Items/0Master_Blueprints/DataAssets/DA_Master_InteractableObjectInfo.DA_Master_InteractableObjectInfo_C|GetName (Variables|Default|GetMIO%20Data%20Asset))) ": Empty Computer Construct Data Asset") "(R=0.000000,G=0.089136,B=1.000000,A=1.000000)" 5.0 "NewEnumerator0"))))

(fn ConstructionScript
  (|CallParentFunction))