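; Master Blueprint for interactable objects, driven by a data asset, with an empty Interaction event.
; Construction and BeginPlay position a keypress prompt widget; BeginPlay also sets its text and color.
; When outlines are enabled, construction creates a dynamic outline material, assigns it as the mesh overlay, then immediately replaces that with M_Blank.
; SetOutlineVisbility shows or hides the outline through the dynamic material's thickness parameter, without changing the overlay.
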(event Custom|Interaction
  (params (Is%20Being%20Held :type Boolean) (Key :type Key%20Structure :default "None")))

(event EventBeginPlay
  (bind _mio_data_asset (Variables|InteractableItemInfo|GetMIO%20Data%20Asset))
  (bind _keypress_prompt_indicator_widget (Variables|Default|GetKeypress%20Prompt%20Indicator%20Widget))
  (CallFunction|SetKeypressPromptTextStyle _keypress_prompt_indicator_widget (Variables|/Game/Interactable_Items/0Master_Blueprints/DataAssets/DA_Master_InteractableObjectInfo.DA_Master_InteractableObjectInfo_C|GetKeypress%20Prompt%20Text _mio_data_asset) (Variables|/Game/Interactable_Items/0Master_Blueprints/DataAssets/DA_Master_InteractableObjectInfo.DA_Master_InteractableObjectInfo_C|GetKeypress%20Prompt%20Color _mio_data_asset))
  (Transformation|SetRelativeLocation _keypress_prompt_indicator_widget (Variables|/Game/Interactable_Items/0Master_Blueprints/DataAssets/DA_Master_InteractableObjectInfo.DA_Master_InteractableObjectInfo_C|GetKeypress%20Prompt%20Overlay%20Location _mio_data_asset) false false))

(fn ConstructionScript
  (bind _object (Variables|Default|GetObject))
  (bind _mio_data_asset (Variables|InteractableItemInfo|GetMIO%20Data%20Asset))
  (bind _object_2 (Variables|Default|GetObject))
  (Transformation|SetRelativeLocation (Variables|Default|GetKeypress%20Prompt%20Indicator%20Widget) (Variables|/Game/Interactable_Items/0Master_Blueprints/DataAssets/DA_Master_InteractableObjectInfo.DA_Master_InteractableObjectInfo_C|GetKeypress%20Prompt%20Overlay%20Location _mio_data_asset) false false)
  (if (Variables|/Game/Interactable_Items/0Master_Blueprints/DataAssets/DA_Master_InteractableObjectInfo.DA_Master_InteractableObjectInfo_C|GetShow%20Object%20Outline _mio_data_asset)
    (bind _returnvalue (Rendering|Material|CreateDynamicMaterialInstance (Variables|/Game/Interactable_Items/0Master_Blueprints/DataAssets/DA_Master_InteractableObjectInfo.DA_Master_InteractableObjectInfo_C|GetOutline%20Material _mio_data_asset) "None" "None" :!class /Script/Engine.KismetMaterialLibrary))
    (bind _output_get (Variables|OutlineSettings|SetGI%20Outline%20MID _returnvalue))
    (Rendering|Material|SetScalarParameterValue _output_get "Outline Thickness" (Variables|/Game/Interactable_Items/0Master_Blueprints/DataAssets/DA_Master_InteractableObjectInfo.DA_Master_InteractableObjectInfo_C|GetOutline%20Thickness _mio_data_asset) :!class /Script/Engine.MaterialInstanceDynamic)
    (Rendering|Material|SetVectorParameterValue _output_get "Outline Color" (Variables|/Game/Interactable_Items/0Master_Blueprints/DataAssets/DA_Master_InteractableObjectInfo.DA_Master_InteractableObjectInfo_C|GetOutline%20Color _mio_data_asset) :!class /Script/Engine.MaterialInstanceDynamic)
    (Rendering|Material|SetOverlayMaterial _object (Variables|OutlineSettings|GetGI%20Outline%20MID) :!class /Script/Engine.MeshComponent)
    (Rendering|Material|SetOverlayMaterial _object "/Game/LevelAssets/A_Main/_Shared/Materials/M_Blank.M_Blank" :!class /Script/Engine.MeshComponent) ; Set material as blank
    (if (Utilities|IsValid _object_2)
      (Variables|OutlineSettings|SetMesh%20To%20Use _object_2))))

(fn SetKeypressPromptTextStyle
  (params (Widget :type Widget%20Component%20Object%20Reference) (Text :type Text) (Color%20and%20Opacity :type Color%20Structure))
  (bind _aswbp_3d_keypress_prompt_indicator (Utilities|Casting|CastToWBP_3D_Keypress_Prompt_Indicator (UserInterface|GetWidget (Variables|Default|GetKeypress%20Prompt%20Indicator%20Widget))))
  (Variables|/Script/UMG.TextBlock|SetText (Variables|/Game/UI/Galactic_Interface/WBP_3D_Keypress_Prompt_Indicator.WBP_3D_Keypress_Prompt_Indicator_C|GetKeyPromptText _aswbp_3d_keypress_prompt_indicator) Text)
  (Variables|/Script/UMG.TextBlock|SetColorAndOpacity (Variables|/Game/UI/Galactic_Interface/WBP_3D_Keypress_Prompt_Indicator.WBP_3D_Keypress_Prompt_Indicator_C|GetKeyPromptText _aswbp_3d_keypress_prompt_indicator) (Utilities|Struct|MakeSlateColor (Math|Conversions|ToLinearColor(Color) Color%20and%20Opacity))))

(fn SetOutlineVisbility
  (params (NewParam :type E_ShowHide%20Enum :default "NewEnumerator0"))
  (Rendering|Material|SetScalarParameterValue (Variables|OutlineSettings|GetGI%20Outline%20MID) "Outline Thickness" (Utilities|Select :Index NewParam :NewEnumerator0 (Variables|/Game/Interactable_Items/0Master_Blueprints/DataAssets/DA_Master_InteractableObjectInfo.DA_Master_InteractableObjectInfo_C|GetOutline%20Thickness (Variables|InteractableItemInfo|GetMIO%20Data%20Asset)) :NewEnumerator1 0.0) :!class /Script/Engine.MaterialInstanceDynamic))