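; Interactable lore node with a glowing tablet material, keypress prompt and progress bar.
; Interaction hides the prompt and runs a progress timeline, which GolemFound can stop while restoring the prompt.
; On completion it turns off the emissive glow and light, fades LoreText through the game controller's UI over LoreTimeOnScreen, and ignores an object trace channel.
; Switches on Area and NodeID follow the timer start but have no actions attached.
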(event Custom|Start%20TImer
  (bind _as_wbp_progress_bar (Variables|References|GetAs%20WBP%20Progress%20Bar))
  (bind _progressbar_0 (Variables|/Game/UI/UI/WBP_ProgressBar.WBP_ProgressBar_C|GetProgressBar_0 _as_wbp_progress_bar))
  (Widget|SetRenderOpacity (Variables|/Game/UI/UI/WBP_3D_Keypress_Prompt_Indicator.WBP_3D_Keypress_Prompt_Indicator_C|GetMainCanvas (Variables|References|GetAs%20WBP%203D%20Keypress%20Prompt%20Indicator)) 0.0)
  (Progress|SetPercent _progressbar_0 0.0)
  (Rendering|SetVisibility (Variables|Default|GetProgressBar) true false)
  (bind _main (Timeline|Progress PlayFromStart)
    (:Update
      (Progress|SetPercent _progressbar_0 _main))
    (:Finished
      (Variables|Internal|SetNodeActivated false)
      (Rendering|Material|SetScalarParameterValue (Variables|Internal|GetGlow%20Material) "Emissive" 0.0 :!class /Script/Engine.MaterialInstanceDynamic)
      (Rendering|Components|Light|SetIntensity (Variables|Default|GetPointLight) 0.0)
      (Rendering|SetVisibility (Variables|Default|GetProgressBar) false false)
      (Components|Timeline|SetPlayRate (Variables|Default|GetLoreFade) (/ 1.0 (Variables|LoreAnimation|GetLore%20Time%20On%20Screen)))
      (bind _returnvalue (Actor|GetActorOfClass "/Game/LevelAssets/Epic/StoryAdvTemplate/Blueprints/BP_GameController_New.BP_GameController_New_C"))
      (Variables|/Script/UMG.TextBlock|SetText (Variables|/Game/UI/UI/WBP_Lore.WBP_Lore_C|GetLore (Variables|/Game/LevelAssets/Epic/StoryAdvTemplate/Blueprints/BP_GameController_New.BP_GameController_New_C|GetLore%20UI _returnvalue)) (Variables|LoreAnimation|GetLoreText))
      (bind _newtrack_0 (Timeline|LoreFade PlayFromStart)
        (:Update
          (Widget|SetRenderOpacity (Variables|/Game/UI/UI/WBP_Lore.WBP_Lore_C|GetCanvasPanel (Variables|/Game/LevelAssets/Epic/StoryAdvTemplate/Blueprints/BP_GameController_New.BP_GameController_New_C|GetLore%20UI _returnvalue)) _newtrack_0)
          (Collision|SetCollisionResponsetoChannel (Variables|Default|GetObject) "ECC_GameTraceChannel1" "ECR_Ignore"))))))

(event Custom|Golem%20Found
  (Widget|SetRenderOpacity (Variables|/Game/UI/UI/WBP_3D_Keypress_Prompt_Indicator.WBP_3D_Keypress_Prompt_Indicator_C|GetMainCanvas (Variables|References|GetAs%20WBP%203D%20Keypress%20Prompt%20Indicator)) 1.0)
  (Utilities|FlowControl|Sequence
    (:then_0
      (if (Audio|Components|Audio|IsPlaying (Variables|Default|GetProgress))
        (bind _main (Timeline|Progress Stop)
          (:Update
            (Progress|SetPercent (Variables|/Game/UI/UI/WBP_ProgressBar.WBP_ProgressBar_C|GetProgressBar_0 (Variables|References|GetAs%20WBP%20Progress%20Bar)) _main))
          (:Finished
            (Variables|Internal|SetNodeActivated false)
            (Rendering|Material|SetScalarParameterValue (Variables|Internal|GetGlow%20Material) "Emissive" 0.0 :!class /Script/Engine.MaterialInstanceDynamic)
            (Rendering|Components|Light|SetIntensity (Variables|Default|GetPointLight) 0.0)
            (Rendering|SetVisibility (Variables|Default|GetProgressBar) false false)
            (Components|Timeline|SetPlayRate (Variables|Default|GetLoreFade) (/ 1.0 (Variables|LoreAnimation|GetLore%20Time%20On%20Screen)))
            (bind _returnvalue (Actor|GetActorOfClass "/Game/LevelAssets/Epic/StoryAdvTemplate/Blueprints/BP_GameController_New.BP_GameController_New_C"))
            (Variables|/Script/UMG.TextBlock|SetText (Variables|/Game/UI/UI/WBP_Lore.WBP_Lore_C|GetLore (Variables|/Game/LevelAssets/Epic/StoryAdvTemplate/Blueprints/BP_GameController_New.BP_GameController_New_C|GetLore%20UI _returnvalue)) (Variables|LoreAnimation|GetLoreText))
            (bind _newtrack_0 (Timeline|LoreFade PlayFromStart)
              (:Update
                (Widget|SetRenderOpacity (Variables|/Game/UI/UI/WBP_Lore.WBP_Lore_C|GetCanvasPanel (Variables|/Game/LevelAssets/Epic/StoryAdvTemplate/Blueprints/BP_GameController_New.BP_GameController_New_C|GetLore%20UI _returnvalue)) _newtrack_0)
                (Collision|SetCollisionResponsetoChannel (Variables|Default|GetObject) "ECC_GameTraceChannel1" "ECR_Ignore")))))))))

(event EventBeginPlay
  (|CallParentFunction)
  (bind _aswbp_3d_keypress_prompt_indicator (Utilities|Casting|CastToWBP_3D_Keypress_Prompt_Indicator (UserInterface|GetWidget (Variables|Default|GetKeypress%20Prompt%20Indicator%20Widget))))
  (Variables|References|SetAs%20WBP%203D%20Keypress%20Prompt%20Indicator _aswbp_3d_keypress_prompt_indicator)
  (bind _aswbp_progress_bar (Utilities|Casting|CastToWBP_ProgressBar (UserInterface|GetWidget (Variables|Default|GetProgressBar))))
  (Variables|References|SetAs%20WBP%20Progress%20Bar _aswbp_progress_bar))

(event Collision|EventActorBeginOverlap
  (params (OtherActor :type Actor%20Object%20Reference))
  (|CallParentFunction OtherActor) ; This node is disabled and will not be called.\nDrag off pins to build functionality.
)

(event EventTick
  (params (DeltaSeconds :type Float%20%28single-precision%29))
  (|CallParentFunction DeltaSeconds) ; This node is disabled and will not be called.\nDrag off pins to build functionality.
)

(event EventInteraction
  (params (Is%20Being%20Held :type Boolean) (Key :type Key%20Structure :default "None"))
  (bind _node_id (Variables|General|GetNode%20ID))
  (|CallParentFunction Is%20Being%20Held Key)
  (if (not (Variables|Internal|GetNodeActivated))
    (CallFunction|StartTImer)
    (switch Utilities|FlowControl|Switch|SwitchonE_GameArea (Variables|General|GetArea)
      (:NewEnumerator0
        (switch int _node_id))
      (:NewEnumerator1
        (switch int _node_id)))))

(fn ConstructionScript
  (|CallParentFunction)
  (bind _returnvalue (Rendering|Material|CreateDynamicMaterialInstance (Variables|Default|GetObject) 1 "/Game/LevelAssets/Internal/Materials/M_TABLET_GLOW.M_TABLET_GLOW" "None" :!class /Script/Engine.PrimitiveComponent))
  (Variables|Internal|SetGlow%20Material _returnvalue))