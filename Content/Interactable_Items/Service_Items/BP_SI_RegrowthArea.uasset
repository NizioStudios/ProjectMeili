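; Interactable regrowth area that fades in foliage from its attached PCG stamp actor and reports to the game controller.
; BeginPlay creates dynamic materials for the stamp's instanced meshes.
; Interaction, if its area type is unfinished, starts the controller's timer, plays a flipbook and drives "FadeA" by timeline, which ReverseFoliageGrowth can reverse.
; On completion, it notifies the controller if all areas sharing its type are regrown.
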(event Custom|Grow%20Foliage
  (bind _self self)
  (bind _areatype (Variables|Public|GetAreaType))
  (bind _paperflipbook (Variables|Default|GetPaperFlipbook))
  ;[0.15 0.15 0.15 0.5] Interact
  (Utilities|FlowControl|Sequence
    (:then_0
      (goto _label Open))
    (:then_1
      (Widget|SetRenderOpacity (UserInterface|GetWidget (Variables|Default|GetKeypress%20Prompt%20Indicator%20Widget)) 0.0)
      (Components|Timeline|SetLooping _paperflipbook false)
      (Components|Timeline|PlayfromStart _paperflipbook)
      (Rendering|SetVisibility _paperflipbook true false)
      (EventDispatchers|BindEventtoOnFinishedPlaying _paperflipbook (delegate Custom|OnFinished))
      (bind (_direction _newtrack_1) (Timeline|Timeline PlayFromStart)
        (:Update
          (for _array_element (Variables|FoliageRegrowth|GetArray%20of%20Materials)
            (for _array_element_2 (.materials _array_element)
              (Rendering|Material|SetScalarParameterValue _array_element_2 "FadeA" _newtrack_1 :!class /Script/Engine.MaterialInstanceDynamic))))
        (:Finished
          (Utilities|FlowControl|Gate true :!label _label
            (:Exit
              (Utilities|FlowControl|Sequence
                (:then_0
                  (Variables|FoliageRegrowth|SetHas%20Area%20Been%20Regrown true)
                  (bind _outactors (Actor|GetAllActorsOfClass "BP_SI_RegrowthArea_C"))
                  (bind _array_element_3 (Utilities|Array|ForEachLoopwithBreak _outactors :!label _label_2)
                    (:LoopBody
                      (if (Utilities|Enum|Equal(Enum) (Variables|BP_SI_RegrowthArea_C|GetAreaType _array_element_3) (Variables|Public|GetAreaType))
                        (if (Variables|BP_SI_RegrowthArea_C|GetHas%20Area%20Been%20Regrown _array_element_3)
                          (Variables|Default|SetHave%20All%20Areas%20Been%20Regrown true)
                          (else
                            (Variables|Default|SetHave%20All%20Areas%20Been%20Regrown false)
                            (Utilities|FlowControl|Sequence
                              (:then_0
                                (goto _label_2 Break))
                              (:then_1
                                (if (Variables|Default|GetHave%20All%20Areas%20Been%20Regrown) :!label _label_3
                                  (CallFunction|PrintDebugData true "All Areas Regrown" "(R=0.000000,G=0.089136,B=1.000000,A=1.000000)" 5.0 "NewEnumerator0")
                                  (bind _returnvalue (Actor|GetActorOfClass "/Game/LevelAssets/Epic/StoryAdvTemplate/Blueprints/BP_GameController_New.BP_GameController_New_C"))
                                  (Default|FinishedRegrowthforArea _returnvalue _areatype)
                                  (switch Utilities|FlowControl|Switch|SwitchonE_GameArea _areatype
                                    (:NewEnumerator0
                                      (CallFunction|PrintDebugData true "Tutorial Regrowth Finished" "(R=0.000000,G=0.089136,B=1.000000,A=1.000000)" 5.0 "NewEnumerator0" _self))
                                    (:NewEnumerator1
                                      (CallFunction|PrintDebugData true "Main Regrowth Finished" "(R=0.000000,G=0.089136,B=1.000000,A=1.000000)" 5.0 "NewEnumerator0" _self)))
                                  (else
                                    (CallFunction|PrintDebugData true "Non All Areas Regrown" "(R=0.000000,G=0.089136,B=1.000000,A=1.000000)" 5.0 "NewEnumerator2")))))))))
                    (:Completed
                      (goto _label_3))))
                (:then_1
                  (Widget|SetRenderOpacity (UserInterface|GetWidget (Variables|Default|GetKeypress%20Prompt%20Indicator%20Widget)) (Utilities|Select :Index _direction :Forward 0.0 :Backward 1.0)))))))))))

(event Custom|ReverseFoliageGrowth
  (bind _self self)
  (bind _areatype (Variables|Public|GetAreaType))
  ;[0.15 0.15 0.15 0.5] Interact
  (Utilities|FlowControl|Sequence
    (:then_0
      (goto _label Close))
    (:then_1
      (bind (_direction _newtrack_1) (Timeline|Timeline Reverse)
        (:Update
          (for _array_element (Variables|FoliageRegrowth|GetArray%20of%20Materials)
            (for _array_element_2 (.materials _array_element)
              (Rendering|Material|SetScalarParameterValue _array_element_2 "FadeA" _newtrack_1 :!class /Script/Engine.MaterialInstanceDynamic))))
        (:Finished
          (Utilities|FlowControl|Gate true :!label _label
            (:Exit
              (Utilities|FlowControl|Sequence
                (:then_0
                  (Variables|FoliageRegrowth|SetHas%20Area%20Been%20Regrown true)
                  (bind _outactors (Actor|GetAllActorsOfClass "BP_SI_RegrowthArea_C"))
                  (bind _array_element_3 (Utilities|Array|ForEachLoopwithBreak _outactors :!label _label_2)
                    (:LoopBody
                      (if (Utilities|Enum|Equal(Enum) (Variables|BP_SI_RegrowthArea_C|GetAreaType _array_element_3) (Variables|Public|GetAreaType))
                        (if (Variables|BP_SI_RegrowthArea_C|GetHas%20Area%20Been%20Regrown _array_element_3)
                          (Variables|Default|SetHave%20All%20Areas%20Been%20Regrown true)
                          (else
                            (Variables|Default|SetHave%20All%20Areas%20Been%20Regrown false)
                            (Utilities|FlowControl|Sequence
                              (:then_0
                                (goto _label_2 Break))
                              (:then_1
                                (if (Variables|Default|GetHave%20All%20Areas%20Been%20Regrown) :!label _label_3
                                  (CallFunction|PrintDebugData true "All Areas Regrown" "(R=0.000000,G=0.089136,B=1.000000,A=1.000000)" 5.0 "NewEnumerator0")
                                  (bind _returnvalue (Actor|GetActorOfClass "/Game/LevelAssets/Epic/StoryAdvTemplate/Blueprints/BP_GameController_New.BP_GameController_New_C"))
                                  (Default|FinishedRegrowthforArea _returnvalue _areatype)
                                  (switch Utilities|FlowControl|Switch|SwitchonE_GameArea _areatype
                                    (:NewEnumerator0
                                      (CallFunction|PrintDebugData true "Tutorial Regrowth Finished" "(R=0.000000,G=0.089136,B=1.000000,A=1.000000)" 5.0 "NewEnumerator0" _self))
                                    (:NewEnumerator1
                                      (CallFunction|PrintDebugData true "Main Regrowth Finished" "(R=0.000000,G=0.089136,B=1.000000,A=1.000000)" 5.0 "NewEnumerator0" _self)))
                                  (else
                                    (CallFunction|PrintDebugData true "Non All Areas Regrown" "(R=0.000000,G=0.089136,B=1.000000,A=1.000000)" 5.0 "NewEnumerator2")))))))))
                    (:Completed
                      (goto _label_3))))
                (:then_1
                  (Widget|SetRenderOpacity (UserInterface|GetWidget (Variables|Default|GetKeypress%20Prompt%20Indicator%20Widget)) (Utilities|Select :Index _direction :Forward 0.0 :Backward 1.0)))))))))))

(event Custom|OnFinished
  ;[0.15 0.15 0.15 0.5] Interact
  (Rendering|SetVisibility (Variables|Default|GetPaperFlipbook) false false))

(event EventBeginPlay
  (bind _returnvalue (Transformation|GetActorLocation))
  (bind _outactors (Actor|GetAttachedActors true false))
  (bind (_x _y) (Math|Vector|BreakVector _returnvalue))
  (bind _output (Utilities|Array|Get(acopy) _outactors))
  (bind _returnvalue_2 (Transformation|GetActorTransform _output))
  (bind _location (Math|Transform|BreakTransform _returnvalue_2))
  (bind (_x_2 _y_2 _z) (Math|Vector|BreakVector _location))
  (|CallParentFunction)
  ;[0.15 0.15 0.15 0.5] Event Begin Play
  (Audio|Components|Audio|Stop (Variables|Default|GetPaperFlipbook))
  (Variables|Default|SetPCG%20Stamp (Variables|/Script/Engine.Actor|GetRootComponent _output))
  (Transformation|SetWorldTransform (Variables|Default|GetBox) _returnvalue_2 false false)
  (Transformation|SetWorldLocation (Variables|Default|GetKeypress%20Prompt%20Indicator%20Widget) (Math|Vector|MakeVector _x_2 _y_2 (/ _z 4.0)) false false)
  (Utilities|FlowControl|Sequence
    (:then_0
      (for (_array_element _array_index) (Components|GetChildrenComponents (Variables|Default|GetPCG%20Stamp) false)
        (bind _asinstanced_static_mesh_component (Utilities|Casting|CastToInstancedStaticMeshComponent _array_element)
          (:then
            (for (_array_element_2 _array_index_2) (Rendering|Material|GetMaterials _asinstanced_static_mesh_component)
              (bind _returnvalue_3 (Rendering|Material|CreateDynamicMaterialInstance _asinstanced_static_mesh_component _array_index_2 _array_element_2 "None" :!class /Script/Engine.PrimitiveComponent)) ; Make Array of arrays for All materials after testing just the trunk on a couple trees
              (Utilities|Array|SetArrayElem (Variables|FoliageRegrowth|GetMaterialDyanmicTest) _array_index_2 _returnvalue_3 true)))
          (:CastFailed
            (bind _asinstanced_static_mesh_component_2 (Utilities|Casting|CastToInstancedStaticMeshComponent _array_element))
            (for (_array_element_3 _array_index_3) (Rendering|Material|GetMaterials _asinstanced_static_mesh_component_2)
              (bind _returnvalue_4 (Rendering|Material|CreateDynamicMaterialInstance _asinstanced_static_mesh_component_2 _array_index_3 _array_element_3 "None" :!class /Script/Engine.PrimitiveComponent)) ; Make Array of arrays for All materials after testing just the trunk on a couple trees
              (Utilities|Array|SetArrayElem (Variables|FoliageRegrowth|GetMaterialDyanmicTest) _array_index_3 _returnvalue_4 true))))
        (Utilities|Array|SetArrayElem (Variables|FoliageRegrowth|GetArray%20of%20Materials) _array_index (Utilities|Struct|MakeST_Material_Array (Variables|FoliageRegrowth|GetMaterialDyanmicTest)) true)))
    (:then_1
      (bind _outhit (Collision|LineTraceByChannel _returnvalue (Math|Vector|MakeVector _x _y -5e+02) "TraceTypeQuery4" true 0 "None" true "(R=1.000000,G=0.000000,B=0.000000,A=1.000000)" "(R=0.000000,G=1.000000,B=0.000000,A=1.000000)" 1.0))
      (Transformation|SetWorldLocation (Variables|Default|GetPaperFlipbook) (Math|Vector|MakeVector (.X (Math|Vector|BreakVector (.ImpactPoint (Collision|BreakHitResult _outhit)))) (.Y (Math|Vector|BreakVector (.ImpactPoint (Collision|BreakHitResult _outhit)))) (+ (.Z (Math|Vector|BreakVector (.ImpactPoint (Collision|BreakHitResult _outhit)))) 1e+01)) false false))))

(event Collision|EventActorBeginOverlap
  (params (OtherActor :type Actor%20Object%20Reference))
  (|CallParentFunction OtherActor) ; This node is disabled and will not be called.\nDrag off pins to build functionality.
)

(event EventTick
  (params (DeltaSeconds :type Float%20%28single-precision%29))
  ;[0.15 0.15 0.15 0.5] Event Begin Play
  (|CallParentFunction DeltaSeconds))

(event EventInteraction
  (params (Is%20Being%20Held :type Boolean) (Key :type Key%20Structure :default "None"))
  ;[0.15 0.15 0.15 0.5] Interact
  (|CallParentFunction Is%20Being%20Held Key)
  (bind _returnvalue (Actor|GetActorOfClass "/Game/LevelAssets/Epic/StoryAdvTemplate/Blueprints/BP_GameController_New.BP_GameController_New_C"))
  (if (not (.Value (Utilities|Map|Find (Variables|/Game/LevelAssets/Epic/StoryAdvTemplate/Blueprints/BP_GameController_New.BP_GameController_New_C|GetAreaMap _returnvalue) (Variables|Public|GetAreaType))))
    (CallFunction|GrowFoliage)
    (bind _returnvalue_2 (Actor|GetActorOfClass "/Game/LevelAssets/Epic/StoryAdvTemplate/Blueprints/BP_GameController_New.BP_GameController_New_C"))
    (Variables|/Game/LevelAssets/Epic/StoryAdvTemplate/Blueprints/BP_GameController_New.BP_GameController_New_C|SetCurrent%20Area _returnvalue_2 (Variables|Public|GetAreaType))
    (Default|StartTimer _returnvalue_2)))

(fn ConstructionScript
  (|CallParentFunction))